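; Player stats component that tracks current and max health and stamina for the third-person character.
; On BeginPlay it caches the player character and initializes its HUD health bar, health text and stamina bar.
; Increase and decrease functions update the values and push them straight to the HUD widget.
; Increases to current values cap at max, while decreases return true when the value reaches zero or below.
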(event `self.ReceiveBeginPlay`
  (bind _hud_widget (`/Game/ThirdPerson/Blueprints/BP_ThirdPersonCharacter.HUD Widget` (`self.Player Character BP`)))
  (bind _asbp_third_person_character (cast `/Game/ThirdPerson/Blueprints/BP_ThirdPersonCharacter` (`GameplayStatics.GetPlayerCharacter` 0)))
  (set `self.Player Character BP` _asbp_third_person_character)
  (`ProgressBar.SetPercent` (`/Game/UI/WB_HUD.StaminaBar` (`/Game/ThirdPerson/Blueprints/BP_ThirdPersonCharacter.HUD Widget` (`self.Player Character BP`))) (/ (`self.CurrentStamina`) (`self.MaxStamina`)))
  (`ProgressBar.SetPercent` (`/Game/UI/WB_HUD.HealthBar` _hud_widget) (/ (`self.CurrentHealth`) (`self.MaxHealth`)))
  (`TextBlock.SetText` (`/Game/UI/WB_HUD.HealthText` _hud_widget) (`KismetTextLibrary.Conv_DoubleToText` (`self.CurrentHealth`) "HalfToEven")))

(fn `Decrease Health`
  (params (Damage :type "Float (double-precision)"))
  (returns (`PlayerDead?` :type Boolean))
  (bind _hud_widget (`/Game/ThirdPerson/Blueprints/BP_ThirdPersonCharacter.HUD Widget` (`self.Player Character BP`)))
  (bind _output_get (set `self.CurrentHealth` (- (`self.CurrentHealth`) Damage)))
  (`ProgressBar.SetPercent` (`/Game/UI/WB_HUD.HealthBar` _hud_widget) (/ _output_get (`self.MaxHealth`)))
  (`TextBlock.SetText` (`/Game/UI/WB_HUD.HealthText` _hud_widget) (`KismetTextLibrary.Conv_DoubleToText` (`self.CurrentHealth`) "HalfToEven"))
  (if (<= (`self.CurrentHealth`) 0.0)
    (return true)
    (else
      (return false))))

(fn `Decrease Stamina`
  (params (`Stamina Depleted` :type "Float (double-precision)"))
  (returns (`No Stamina` :type Boolean))
  (set `self.CurrentStamina` (- (`self.CurrentStamina`) `Stamina Depleted`))
  (`ProgressBar.SetPercent` (`/Game/UI/WB_HUD.StaminaBar` (`/Game/ThirdPerson/Blueprints/BP_ThirdPersonCharacter.HUD Widget` (`self.Player Character BP`))) (/ (`self.CurrentStamina`) (`self.MaxStamina`)))
  (if (<= (`self.CurrentStamina`) 0.0)
    (return true)
    (else
      (return false))))

(fn `Increase Health`
  (params (`Added Health` :type "Float (double-precision)"))
  (bind _hud_widget (`/Game/ThirdPerson/Blueprints/BP_ThirdPersonCharacter.HUD Widget` (`self.Player Character BP`)))
  (set `self.CurrentHealth` (+ (`self.CurrentHealth`) `Added Health`))
  (if (> (`self.CurrentHealth`) (`self.MaxHealth`))
    (set `self.CurrentHealth` (`self.MaxHealth`)))
  (`ProgressBar.SetPercent` (`/Game/UI/WB_HUD.HealthBar` _hud_widget) (/ (`self.CurrentHealth`) (`self.MaxHealth`)))
  (`TextBlock.SetText` (`/Game/UI/WB_HUD.HealthText` _hud_widget) (`KismetTextLibrary.Conv_DoubleToText` (`self.CurrentHealth`) "HalfToEven")))

(fn `Increase Max Health`
  (params (HealthIncrease :type "Float (double-precision)"))
  (bind _hud_widget (`/Game/ThirdPerson/Blueprints/BP_ThirdPersonCharacter.HUD Widget` (`self.Player Character BP`)))
  (set `self.MaxHealth` (+ (`self.MaxHealth`) HealthIncrease))
  (`ProgressBar.SetPercent` (`/Game/UI/WB_HUD.HealthBar` _hud_widget) (/ (`self.CurrentHealth`) (`self.MaxHealth`)))
  (`TextBlock.SetText` (`/Game/UI/WB_HUD.HealthText` _hud_widget) (`KismetTextLibrary.Conv_DoubleToText` (`self.CurrentHealth`) "HalfToEven")))

(fn `Increase Max Stamina`
  (params (StaminaIncrease :type "Float (double-precision)"))
  (set `self.MaxStamina` (+ (`self.MaxStamina`) StaminaIncrease))
  (`ProgressBar.SetPercent` (`/Game/UI/WB_HUD.StaminaBar` (`/Game/ThirdPerson/Blueprints/BP_ThirdPersonCharacter.HUD Widget` (`self.Player Character BP`))) (/ (`self.CurrentStamina`) (`self.MaxStamina`))))

(fn `Increase Stamina`
  (params (`Added Stamina` :type "Float (double-precision)"))
  (set `self.CurrentStamina` (+ (`self.CurrentStamina`) `Added Stamina`))
  (if (> (`self.CurrentStamina`) (`self.MaxStamina`))
    (set `self.CurrentStamina` (`self.MaxStamina`)))
  (`ProgressBar.SetPercent` (`/Game/UI/WB_HUD.StaminaBar` (`/Game/ThirdPerson/Blueprints/BP_ThirdPersonCharacter.HUD Widget` (`self.Player Character BP`))) (/ (`self.CurrentStamina`) (`self.MaxStamina`))))