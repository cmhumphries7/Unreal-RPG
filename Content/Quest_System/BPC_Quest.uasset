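; Quest component that shows the active quest on a HUD and tracks its enemy-elimination objectives.
; It creates WB_QuestHUD on BeginPlay, with events to push the quest name and objectives into it.
; EliminateEnemy removes the enemy from a working array, seeded from the objective when empty, and writes it back by reference.
; An emptied array completes the objective on the HUD; chest objective fields are only carried through.
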(event `self.ReceiveBeginPlay`
  (bind _returnvalue (`|CreateWidget` "/Game/Quest_System/WB_QuestHUD.WB_QuestHUD_C"))
  (bind _output_get (set `self.Quest HUD Widget` _returnvalue))
  (`UserWidget.AddToViewport` _output_get 0))

(event `Set Active Quest Text`
  (bind _activequest_name (break `/Game/Quest_System/S_Quest` (`self.activeQuest`)))
  (`TextBlock.SetText` (`/Game/Quest_System/WB_QuestHUD.ActiveQuestText` (`self.Quest HUD Widget`)) (`KismetTextLibrary.Conv_StringToText` _activequest_name)))

(event `Set Objectives`
  (bind (_activequest_name _activequest_description _activequest_secondary _activequest_completed _activequest_objectives) (break `/Game/Quest_System/S_Quest` (`self.activeQuest`)))
  (`/Game/Quest_System/WB_QuestHUD.Populate Objectives` (`self.Quest HUD Widget`) _activequest_objectives))

(event `Eliminate Enemy`
  (params (`Enemy Eliminated` :type "Actor Object Reference"))
  (bind (_activequest_name _activequest_description _activequest_secondary _activequest_completed _activequest_objectives) (break `/Game/Quest_System/S_Quest` (`self.activeQuest`)))
  (for _array_element _activequest_objectives
    (bind (_nameaim _completed _actorstoeliminate _chesttoopen _iseliminateenemyobjective _ischestobjective) (break `/Game/Quest_System/S_QuestObjectives` _array_element))
    (if (and (not _completed) _iseliminateenemyobjective)
      (if (not (!= (`KismetArrayLibrary.Array_Length` (`self.enemy actors array`)) 0))
        (bind _output_get (set `self.enemy actors array` _actorstoeliminate)))
      (`KismetArrayLibrary.Array_RemoveItem` _output_get `Enemy Eliminated`)
      (`|VariableSetRef` _array_element (make `/Game/Quest_System/S_QuestObjectives` _nameaim false (`self.enemy actors array`) _chesttoopen _iseliminateenemyobjective _ischestobjective))
      (bind _returnvalue (`KismetArrayLibrary.Array_Length` _output_get))
      (`KismetSystemLibrary.PrintString` (`KismetStringLibrary.Conv_IntToString` _returnvalue))
      (if (== _returnvalue 0)
        (`|VariableSetRef` _array_element (make `/Game/Quest_System/S_QuestObjectives` _nameaim true _ _chesttoopen _iseliminateenemyobjective _ischestobjective))
        (`/Game/Quest_System/WB_QuestHUD.Complete Objective` (`self.Quest HUD Widget`) _array_element)
        (`KismetSystemLibrary.PrintString` "Completed")))))